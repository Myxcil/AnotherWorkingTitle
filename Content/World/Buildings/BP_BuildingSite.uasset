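; BP_BuildingSite is a building site that displays its construction progress and missing resources on a debug widget.
; On BeginPlay it caches the WBP_DebugProgress from its widget component, binds to the building progress and build cost update events, then initializes the display.
; Two update functions push progress and missing resources into the widget when it is valid.
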(event `self.ReceiveBeginPlay`
  (bind _aswbp_debug_progress (cast `/Game/UI/HUD/WBP_DebugProgress` (`WidgetComponent.GetUserWidgetObject` (`self.BP_DebugWidgetComponent`))))
  (set `self.ProgressWidget` _aswbp_debug_progress)
  (add `self.OnBuildingProgress` (`|CreateDelegate` :!event `UpdateBuildProgress`))
  (add `self.OnBuildCostUpdated` (`|CreateDelegate` :!event `UpdateBuildCost`))
  (`self.UpdateBuildProgress` 0.0)
  (`self.UpdateBuildCost` _))

(fn `UpdateBuildCost`
  (params (Missing :type "Array of ResourceAmount Structure (by ref)"))
  (bind _progresswidget (`self.ProgressWidget`))
  (`/Engine/EditorBlueprintResources/StandardMacros.IsValid` _progresswidget
    (:`Is Valid`
      (`/Game/UI/HUD/WBP_DebugProgress.SetMissingResources` _progresswidget Missing)
      (return))))

(fn `UpdateBuildProgress`
  (params (Progress :type "Float (single-precision)"))
  (bind _progresswidget (`self.ProgressWidget`))
  (`/Engine/EditorBlueprintResources/StandardMacros.IsValid` _progresswidget
    (:`Is Valid`
      (set `/Game/UI/HUD/WBP_DebugProgress.Progress` Progress _progresswidget))))

(fn `UserConstructionScript`)