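; Debug widget component that shows itself only while the player is near its owning actor.
; BeginPlay caches the player pawn as a SettlerCharacter.
; Each Tick, if that reference is valid, it compares the player's distance to the owner against ViewDistance and sets visibility accordingly, propagating to child components.
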(event `self.ReceiveBeginPlay`
  (bind _assettler_character (cast `SettlerCharacter` (`GameplayStatics.GetPlayerPawn` 0)))
  (set `self.PlayerCharacter` _assettler_character))

(event `self.ReceiveTick`
  (params (DeltaSeconds :type "Float (single-precision)"))
  (bind _playercharacter (`self.PlayerCharacter`))
  (`/Engine/EditorBlueprintResources/StandardMacros.IsValid` _playercharacter
    (:`Is Valid`
      (`self.SetVisibility` (<= (`Actor.GetDistanceTo` _playercharacter (`self.GetOwner` self)) (`self.ViewDistance`)) true))))